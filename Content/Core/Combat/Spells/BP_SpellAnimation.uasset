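; BP_SpellAnimation is a short-lived actor that plays the visual for a spell going between two tiles on the combat grid.
; On BeginPlay it spawns a dark red BP_AnimatedShape using the grid's current shape mesh and material, passing it the origin and target tile transforms.
; When that shape signals completion, it broadcasts OnSpellAnimationCompleted and destroys itself.
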(event Custom|Even_PlaySplitAnimation
  (bind _grid (Variables|Default|GetGrid))
  (bind _returnvalue (Default|GetCurrentShapeData _grid))
  (bind (_meshsize _mesh _meshmaterial) (Utilities|Struct|BreakS_GridShapeData _returnvalue))
  (bind _returnvalue_2 (Game|SpawnActorfromClass "/Game/Core/Combat/Spells/Components/BP_AnimatedShape.BP_AnimatedShape_C" (Math|Transform|MakeTransform "0, 0, 0" "0, 0, 0" "1.000000,1.000000,1.000000") "AlwaysSpawn" "MultiplyWithRoot" 0 _mesh _meshmaterial "(R=0.583333,G=0.000000,B=0.000000,A=1.000000)" (CallFunction|GetTileTransform (Variables|Default|GetOriginIndex)) (CallFunction|GetTileTransform (Variables|Default|GetTargetIndex)) 0))
  (EventDispatchers|BindEventtoOnShapeAnimationCompleted _returnvalue_2 (delegate Custom|On%20Shape%20Animation%20Complete)))

(event Custom|On%20Shape%20Animation%20Complete
  (params (AnimatedShape :type BP%20Animated%20Shape%20Object%20Reference))
  (CallFunction|EventCompleteSpellAnimation))

(event Custom|Event_CompleteSpellAnimation
  (Default|CallOnSpellAnimationCompleted self)
  (Actor|DestroyActor))

(event EventBeginPlay
  (CallFunction|EvenPlaySplitAnimation))

(fn ConstructionScript)

(fn GetTileTransform
  (params (Index :type Int%20Point%20Structure%20%28by%20ref%29))
  (return (.Transform (Utilities|Struct|BreakS_TileData (.Value (Utilities|Map|Find (Variables|/Game/Core/Grid/BP_Grid.BP_Grid_C|GetGridTiles (Variables|Default|GetGrid)) Index))))))