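; Grid pathfinder that runs A* between two tiles, or can return the analysed tiles as a reachable set within a max path length.
; Neighbours are filtered by tile type, occupancy and height step, and weighted by terrain cost.
; A cost-sorted open list breaks ties toward straight moves, and GeneratePath walks previous-tile links back.
; Searches run instantly or time-sliced via delay and per-frame millisecond budget, reporting progress and results through callbacks.
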(event Custom|FindPathWithDelay
  (Utilities|FlowControl|Sequence
    (:then_0
      (goto _label_3 Open))
    (:then_1
      (Variables|GeneratedData|SetLoopStartTime (Math|DateTime|Now) :!label _label)
      (if (> (Utilities|Array|Length (Variables|GeneratedData|GetDiscoveredTileIndexes)) 0) :!label _label_2
        (bind _foundtargettile (CallFunction|AnalyzeNextDiscoveredTile))
        (if _foundtargettile
          (bind _path (Utilities|GeneratePath))
          (Default|CallOnPathfindingCompleted _path)
          (else
            (if (> (Variables|Default|GetMaxMsPerFrame) 0.0)
              (if (< (Class|KismetMathLibrary|GetTotalMilliseconds (- (Math|DateTime|Now) (Variables|GeneratedData|GetLoopStartTime))) (Variables|Default|GetMaxMsPerFrame))
                (goto _label_2)
                (else
                  _)))
            (Utilities|FlowControl|RetriggerableDelay (Variables|Default|GetDelayBetweenIterations))
            (Utilities|FlowControl|Gate true :!label _label_3
              (:Exit
                (goto _label)))))
        (else
          (Default|CallOnPathfindingCompleted (select (Variables|Default|GetReturn%20Reachable%20Tiles) (Variables|GeneratedData|GetAnalysedTileIndexes) (Utilities|Array|MakeArray ""))))))))

(event Custom|CloseDelayGate
  (Utilities|FlowControl|Gate true) ; enters at Close
)

(fn ConstructionScript)

(fn GetValidTileNeighbours
  (params (Index :type Int%20Point%20Structure) (IncludeDiagonals :type Boolean) (ValidTypes :type Array%20of%20E_TileType%20Enums :default "NewEnumerator0"))
  (LocalVariables|SetInputData (.Value (Utilities|Map|Find (Variables|/Game/Core/Grid/BP_Grid.BP_Grid_C|GetGridTiles (Variables|Default|GetGrid)) Index)))
  (for _array_element (Neighbours|GetNeighbourIndexes Index IncludeDiagonals)
    (LocalVariables|SetData (.Value (Utilities|Map|Find (Variables|/Game/Core/Grid/BP_Grid.BP_Grid_C|GetGridTiles (Variables|Default|GetGrid)) _array_element)))
    (if (Utilities|Array|ContainsItem ValidTypes (.type (LocalVariables|GetData)))
      (if (not (Utilities|IsValid (.unitontile (LocalVariables|GetData))))
        (if (<= (Math|Float|Absolute(Float) (- (.z (.location (.transform (LocalVariables|GetData)))) (.z (.location (.transform (LocalVariables|GetInputData)))))) (.z (Variables|/Game/Core/Grid/BP_Grid.BP_Grid_C|GetGridTileSize (Variables|Default|GetGrid))))
          (Utilities|Array|Add (LocalVariables|GetRet) (Utilities|Struct|MakeS_PathfindingData (.index (LocalVariables|GetData)) (Utilities|Select :Index (.type (LocalVariables|GetData)) :NewEnumerator0 0 :NewEnumerator1 1 :NewEnumerator2 0 :NewEnumerator3 2 :NewEnumerator4 3 :NewEnumerator5 1) 999999 999999 Index))))))
  (return (LocalVariables|GetRet)))

(fn GetNeighbourIndexes
  (params (Index :type Int%20Point%20Structure) (IncludeDiagonals :type Boolean))
  (bind _intpoint (Utilities|Struct|MakeIntPoint 1 0))
  (bind _intpoint_2 (Utilities|Struct|MakeIntPoint 0 1))
  (bind _intpoint_3 (Utilities|Struct|MakeIntPoint -1 0))
  (bind _intpoint_4 (Utilities|Struct|MakeIntPoint 0 -1))
  (bind _returnvalue (+ Index _intpoint))
  (bind _returnvalue_2 (+ Index _intpoint_2))
  (bind _returnvalue_3 (+ Index _intpoint_3))
  (bind _returnvalue_4 (+ Index _intpoint_4))
  (bind _array (Utilities|Array|MakeArray _returnvalue _returnvalue_2 _returnvalue_3 _returnvalue_4))
  (if IncludeDiagonals
    (bind _output_get (LocalVariables|SetRet _array))
    (Utilities|Array|AppendArray _output_get (Utilities|Array|MakeArray (+ Index (Utilities|Struct|MakeIntPoint 1 1)) (+ Index (Utilities|Struct|MakeIntPoint -1 1)) (+ Index (Utilities|Struct|MakeIntPoint -1 -1)) (+ Index (Utilities|Struct|MakeIntPoint 1 -1))))
    (return (LocalVariables|GetRet))
    (else
      (return _array))))

(fn FindPath
  (params (Start :type Int%20Point%20Structure) (Target :type Int%20Point%20Structure) (Diagonals :type Boolean) (TileTypes :type Array%20of%20E_TileType%20Enums :default "NewEnumerator0") (Delay :type Float%20%28double-precision%29) (MaxMs :type Float%20%28double-precision%29) (ReturnReachables :type Boolean) (PathLength :type Integer))
  (bind _array (Utilities|Array|MakeArray))
  (Variables|PathfindingStartValues|SetStartIndex Start)
  (Variables|PathfindingStartValues|SetTargetIndex Target)
  (Variables|Default|SetIncludeDiagonals Diagonals)
  (Variables|Default|SetValidTileTypes TileTypes)
  (Variables|Default|SetDelayBetweenIterations Delay)
  (Variables|Default|SetMaxMsPerFrame MaxMs)
  (Variables|Default|SetReturn%20Reachable%20Tiles ReturnReachables)
  (Variables|Default|SetMax%20Path%20Length PathLength)
  (CallFunction|CloseDelayGate)
  (Utilities|ClearGeneratedData)
  (Utilities|IsInputDataValid)
  (if true
    (Utilities|DiscoverTile (Utilities|Struct|MakeS_PathfindingData (Variables|PathfindingStartValues|GetStartIndex) 1 0 (Utilities|GetMinimumCostBetweenTwoTiles (Variables|PathfindingStartValues|GetStartIndex) (Variables|PathfindingStartValues|GetTargetIndex) (Variables|Default|GetIncludeDiagonals)) "(X=-999,Y=-999)"))
    (if (<= (Variables|Default|GetDelayBetweenIterations) 0.0)
      (while (> (Utilities|Array|Length (Variables|GeneratedData|GetDiscoveredTileIndexes)) 0)
        (bind _foundtargettile (CallFunction|AnalyzeNextDiscoveredTile))
        (if _foundtargettile
          (bind _path (Utilities|GeneratePath))
          (Default|CallOnPathfindingCompleted _path)
          (return _path)))
      (Default|CallOnPathfindingCompleted (select (Variables|Default|GetReturn%20Reachable%20Tiles) (Variables|GeneratedData|GetAnalysedTileIndexes) (Utilities|Array|MakeArray)))
      (return (select (Variables|Default|GetReturn%20Reachable%20Tiles) (Variables|GeneratedData|GetAnalysedTileIndexes) (Utilities|Array|MakeArray)))
      (else
        (CallFunction|FindPathwithDelay)
        (return (Utilities|Array|MakeArray))))
    (else
      (Default|CallOnPathfindingCompleted _array)
      (return _array))))

(fn ClearGeneratedData
  (Utilities|Map|Clear (Variables|GeneratedData|GetPathfindingData))
  (Utilities|Array|Clear (Variables|GeneratedData|GetDiscoveredTileSortingCosts))
  (Utilities|Array|Clear (Variables|GeneratedData|GetDiscoveredTileIndexes))
  (Utilities|Array|Clear (Variables|GeneratedData|GetAnalysedTileIndexes))
  (Default|CallOnPathfindingDataCleared))

(fn IsInputDataValid
  (bind _grid (Variables|Default|GetGrid))
  (bind _targetindex (Variables|PathfindingStartValues|GetTargetIndex))
  (bind _gridtiles (Variables|/Game/Core/Grid/BP_Grid.BP_Grid_C|GetGridTiles _grid))
  (bind _value (Utilities|Map|Find _gridtiles _targetindex))
  (bind (_index _type _transform _states _unitontile) (Utilities|Struct|BreakS_TileData _value))
  (if (!= (Variables|PathfindingStartValues|GetStartIndex) (Variables|PathfindingStartValues|GetTargetIndex))
    (if (Default|IsTileWalkable (Variables|Default|GetGrid) (Variables|PathfindingStartValues|GetStartIndex))
      (if (not (Variables|Default|GetReturn%20Reachable%20Tiles))
        (if (Default|IsTileWalkable (Variables|Default|GetGrid) (Variables|PathfindingStartValues|GetTargetIndex))
          (if (<= (Utilities|GetMinimumCostBetweenTwoTiles (Variables|PathfindingStartValues|GetStartIndex) (Variables|PathfindingStartValues|GetTargetIndex) (Variables|Default|GetIncludeDiagonals)) (Variables|Default|GetMax%20Path%20Length))
            (if (Utilities|Array|ContainsItem (Variables|Default|GetValidTileTypes) _type)
              (if (not (Utilities|IsValid _unitontile))
                (return true)
                (else
                  _)))
            (return false)
            (else
              (return false)))
          (else
            (return false)))
        (else
          (return true)))
      (else
        (return false)))
    (else
      (return false))))

(fn DiscoverTile
  (params (TilePathData :type S%20Pathfinding%20Data%20Structure))
  (bind _index (Utilities|Struct|BreakS_PathfindingData TilePathData))
  (Utilities|Map|Add (Variables|GeneratedData|GetPathfindingData) _index TilePathData)
  (Utilities|InsertTileinDiscoveredArray TilePathData)
  (Default|CallOnPathfindingDataUpdated _index))

(fn GetMinimumCostBetweenTwoTiles
  (params (Index1 :type Int%20Point%20Structure) (Index2 :type Int%20Point%20Structure) (Diagonals :type Boolean))
  (bind _returnvalue (- Index1 Index2))
  (bind _returnvalue_2 (- Index1 Index2))
  (if Diagonals
    (return (Math|Integer|Max(Integer) (Math|Integer|Absolute(Integer) (.x _returnvalue_2)) (Math|Integer|Absolute(Integer) (.y _returnvalue_2))))
    (else
      (return (+ (Math|Integer|Absolute(Integer) (.x _returnvalue)) (Math|Integer|Absolute(Integer) (.y _returnvalue)))))))

(fn AnalyzeNextDiscoveredTile
  (bind _tilepathdata (Utilities|PullCheapestTileOutOfDiscoveredList))
  (bind _output_get (Variables|GeneratedData|SetCurrentDiscoveredTile _tilepathdata))
  (Default|CallOnPathfindingDataUpdated (.Index (Utilities|Struct|BreakS_PathfindingData _output_get)))
  (bind _neighbours (Neighbours|GetValidTileNeighbours (.Index (Utilities|Struct|BreakS_PathfindingData (Variables|GeneratedData|GetCurrentDiscoveredTile))) (Variables|Default|GetIncludeDiagonals) (Variables|Default|GetValidTileTypes)))
  (Variables|GeneratedData|SetCurrentNeighbours _neighbours)
  (while (> (Utilities|Array|Length (Variables|GeneratedData|GetCurrentNeighbours)) 0)
    (bind _istargettile (CallFunction|DiscoverNextNeighbour))
    (if _istargettile
      (return true)))
  (return false))

(fn GeneratePath
  (LocalVariables|SetCurrent (Variables|PathfindingStartValues|GetTargetIndex))
  (while (!= (LocalVariables|GetCurrent) (Variables|PathfindingStartValues|GetStartIndex))
    (Utilities|Array|Add (LocalVariables|GetInvertedPath) (LocalVariables|GetCurrent))
    (LocalVariables|SetCurrent (.PreviousIndex (Utilities|Struct|BreakS_PathfindingData (.Value (Utilities|Map|Find (Variables|GeneratedData|GetPathfindingData) (LocalVariables|GetCurrent)))))))
  (bind _arrayelement (Utilities|Array|ReverseforEachLoop (LocalVariables|GetInvertedPath))
    (:LoopBody
      (Utilities|Array|Add (LocalVariables|GetRet) _arrayelement))
    (:Completed
      (return (LocalVariables|GetRet)))))

(fn PullCheapestTileOutOfDiscoveredList
  (LocalVariables|SetTileIndex (Utilities|Array|Get(acopy) (Variables|GeneratedData|GetDiscoveredTileIndexes)))
  (Utilities|Array|RemoveIndex (Variables|GeneratedData|GetDiscoveredTileSortingCosts))
  (Utilities|Array|RemoveIndex (Variables|GeneratedData|GetDiscoveredTileIndexes))
  (Utilities|Array|Add (Variables|GeneratedData|GetAnalysedTileIndexes) (LocalVariables|GetTileIndex))
  (return (.Value (Utilities|Map|Find (Variables|GeneratedData|GetPathfindingData) (LocalVariables|GetTileIndex)))))

(fn DiscoverNextNeighbour
  (Variables|GeneratedData|SetCurrentNeighbour (Utilities|Array|Get(acopy) (Variables|GeneratedData|GetCurrentNeighbours)))
  (Utilities|Array|RemoveIndex (Variables|GeneratedData|GetCurrentNeighbours))
  (if (not (Utilities|Array|ContainsItem (Variables|GeneratedData|GetAnalysedTileIndexes) (.Index (Utilities|Struct|BreakS_PathfindingData (Variables|GeneratedData|GetCurrentNeighbour)))))
    (LocalVariables|SetCostFromStart (+ (.CostFromStart (Utilities|Struct|BreakS_PathfindingData (Variables|GeneratedData|GetCurrentDiscoveredTile))) (.CostToEnterTile (Utilities|Struct|BreakS_PathfindingData (Variables|GeneratedData|GetCurrentNeighbour)))))
    (if (<= (LocalVariables|GetCostFromStart) (Variables|Default|GetMax%20Path%20Length))
      (bind _output_get (LocalVariables|SetIndexInDiscovered (Utilities|Array|FindItem (Variables|GeneratedData|GetDiscoveredTileIndexes) (.Index (Utilities|Struct|BreakS_PathfindingData (Variables|GeneratedData|GetCurrentNeighbour))))))
      (if (== _output_get -1)
        _
        (else
          (bind _output_get_2 (Variables|GeneratedData|SetCurrentNeighbour (.Value (Utilities|Map|Find (Variables|GeneratedData|GetPathfindingData) (.Index (Utilities|Struct|BreakS_PathfindingData (Variables|GeneratedData|GetCurrentNeighbour)))))))
          (if (< (LocalVariables|GetCostFromStart) (.CostToEnterTile (Utilities|Struct|BreakS_PathfindingData _output_get_2)))
            (Utilities|Array|RemoveIndex (Variables|GeneratedData|GetDiscoveredTileIndexes) (LocalVariables|GetIndexInDiscovered))
            (Utilities|Array|RemoveIndex (Variables|GeneratedData|GetDiscoveredTileSortingCosts) (LocalVariables|GetIndexInDiscovered))
            (else
              (return false)))))
      (Utilities|DiscoverTile (Utilities|Struct|MakeS_PathfindingData (.Index (Utilities|Struct|BreakS_PathfindingData (Variables|GeneratedData|GetCurrentNeighbour))) (.CostToEnterTile (Utilities|Struct|BreakS_PathfindingData (Variables|GeneratedData|GetCurrentNeighbour))) (LocalVariables|GetCostFromStart) (Utilities|GetMinimumCostBetweenTwoTiles (.Index (Utilities|Struct|BreakS_PathfindingData (Variables|GeneratedData|GetCurrentNeighbour))) (Variables|PathfindingStartValues|GetTargetIndex) (Variables|Default|GetIncludeDiagonals)) (.Index (Utilities|Struct|BreakS_PathfindingData (Variables|GeneratedData|GetCurrentDiscoveredTile)))))
      (if (Class|KismetMathLibrary|EqualIntPointIntPoint (.Index (Utilities|Struct|BreakS_PathfindingData (Variables|GeneratedData|GetCurrentNeighbour))) (Variables|PathfindingStartValues|GetTargetIndex))
        (return true)
        (else
          (return false)))
      (else
        (return false)))
    (else
      (return false))))

(fn InsertTileinDiscoveredArray
  (params (Tile%20Data :type S%20Pathfinding%20Data%20Structure))
  (bind _discoveredtilesortingcosts (Variables|GeneratedData|GetDiscoveredTileSortingCosts))
  (LocalVariables|SetSortingCost (Utilities|GetTileSortingCost Tile%20Data))
  (if (== (Utilities|Array|Length (Variables|GeneratedData|GetDiscoveredTileSortingCosts)) 0)
    (Utilities|Array|Add (Variables|GeneratedData|GetDiscoveredTileSortingCosts) (LocalVariables|GetSortingCost) :!label _label)
    (Utilities|Array|Add (Variables|GeneratedData|GetDiscoveredTileIndexes) (.Index (Utilities|Struct|BreakS_PathfindingData Tile%20Data)))
    (elif (>= (LocalVariables|GetSortingCost) (Utilities|Array|Get(acopy) _discoveredtilesortingcosts (Utilities|Array|LastIndex _discoveredtilesortingcosts)))
      (goto _label)
      (else
        (bind (_array_element _array_index) (Utilities|Array|ForEachLoopwithBreak (Variables|GeneratedData|GetDiscoveredTileSortingCosts) :!label _label_2)
          (:LoopBody
            (if (>= _array_element (LocalVariables|GetSortingCost))
              (Utilities|Array|Insert (Variables|GeneratedData|GetDiscoveredTileSortingCosts) (LocalVariables|GetSortingCost) _array_index)
              (Utilities|Array|Insert (Variables|GeneratedData|GetDiscoveredTileIndexes) (.Index (Utilities|Struct|BreakS_PathfindingData Tile%20Data)) _array_index)
              (goto _label_2 Break))))))))

(fn IsDiagonal
  (params (Index1 :type Int%20Point%20Structure) (Index2 :type Int%20Point%20Structure))
  (return (not (Utilities|Array|ContainsItem (Neighbours|GetNeighbourIndexes Index1 false) Index2))))

(fn GetTileSortingCost
  (params (TileData :type S%20Pathfinding%20Data%20Structure%20%28by%20ref%29))
  (bind (_index _costtoentertile _costfromstart _minimumcosttotarget) (Utilities|Struct|BreakS_PathfindingData TileData))
  (bind (_index_2 _costtoentertile_2 _costfromstart_2 _minimumcosttotarget_2 _previousindex) (Utilities|Struct|BreakS_PathfindingData TileData))
  (return (+ (* (+ _costfromstart _minimumcosttotarget) 2) (Math|Conversions|ToInteger(Boolean) (Utilities|IsDiagonal _index_2 _previousindex)))))