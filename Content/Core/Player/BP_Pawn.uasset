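; Player pawn that acts as a combat camera with move, zoom and yaw rotation controls.
; On begin play it adds the combat camera input mapping and seeds desired location, zoom and rotation from the current state.
; Enhanced Input actions update those targets, with zoom clamped and rotation gated behind holding the right mouse button.
; Tick smoothly interpolates actor transform and spring arm length toward the targets.
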(event Input|EnhancedActionEvents|EnhancedInputActionIA_Zoom
  (params (ActionValue :type Float%20%28double-precision%29) (ElapsedSeconds :type Float%20%28double-precision%29) (TriggeredSeconds :type Float%20%28double-precision%29) (InputAction :type Input%20Action%20Object%20Reference :default "/Game/Core/Input/Actions/IA_Zoom.IA_Zoom"))
  (Variables|Zoom|SetZoom_Desired (Math|Float|Clamp(Float) (+ (* ActionValue (Variables|Zoom|GetZoom_Speed)) (Variables|Zoom|GetZoom_Desired)) (Variables|Zoom|GetZoom_Min) (Variables|Zoom|GetZoom_Max))))

(event Input|EnhancedActionEvents|EnhancedInputActionIA_RotateCam
  (params (ActionValue :type Vector%202D%20Structure) (ElapsedSeconds :type Float%20%28double-precision%29) (TriggeredSeconds :type Float%20%28double-precision%29) (InputAction :type Input%20Action%20Object%20Reference :default "/Game/Core/Input/Actions/IA_RotateCam.IA_RotateCam"))
  (Utilities|FlowControl|Gate true
    (:Exit
      (Variables|Rotation|SetRotation_Desired (Math|Rotator|CombineRotators (Variables|Rotation|GetRotation_Desired) (Math|Rotator|MakeRotator 0.0 0.0 (/ (* (.x ActionValue) (Variables|Rotation|GetRotation_Speed)) 1e+01)))))))

(event Input|EnhancedActionEvents|EnhancedInputActionIA_Move
  (params (ActionValue :type Vector%202D%20Structure) (ElapsedSeconds :type Float%20%28double-precision%29) (TriggeredSeconds :type Float%20%28double-precision%29) (InputAction :type Input%20Action%20Object%20Reference :default "/Game/Core/Input/Actions/IA_Move.IA_Move"))
  (Variables|Location|SetLocation_Desired (+ (Variables|Location|GetLocation_Desired) (+ (* (* (.x ActionValue) (Variables|Location|GetLocation_Speed)) (Transformation|GetActorForwardVector)) (* (* (.y ActionValue) (Variables|Location|GetLocation_Speed)) (Transformation|GetActorRightVector))))))

(event EventTick
  (params (DeltaSeconds :type Float%20%28single-precision%29))
  (bind _springarm (Variables|Default|GetSpringArm))
  ;[0 0 0] ZOOM
  (Variables|/Script/Engine.SpringArmComponent|SetTargetArmLength _springarm (Math|Interpolation|FInterpTo (Variables|/Script/Engine.SpringArmComponent|GetTargetArmLength _springarm) (Variables|Zoom|GetZoom_Desired) (Utilities|Time|GetWorldDeltaSeconds) (Variables|Zoom|GetZoom_Interp)))
  ;[0 0 0] LOCATION
  (Transformation|SetActorLocation (Math|Interpolation|VInterpTo (Transformation|GetActorLocation) (Variables|Location|GetLocation_Desired) (Utilities|Time|GetWorldDeltaSeconds) (Variables|Location|GetLocation_Interp)) false false)
  ;[0 0 0] ROTATION
  (Transformation|SetActorRotation (Math|Interpolation|RInterpTo (Transformation|GetActorRotation) (Variables|Rotation|GetRotation_Desired) (Utilities|Time|GetWorldDeltaSeconds) (Variables|Rotation|GetRotation_Interp))))

(event EventBeginPlay
  (bind _asplayer_controller (Utilities|Casting|CastToPlayerController (Pawn|GetController)))
  (Utilities|IsValid (PlayerController|LocalPlayerSubsystems|GetEnhancedInputLocalPlayerSubsystem _asplayer_controller)
    (:Is%20Valid
      (Input|AddMappingContext (PlayerController|LocalPlayerSubsystems|GetEnhancedInputLocalPlayerSubsystem _asplayer_controller) "/Game/Core/Input/IMC_CombatCamera.IMC_CombatCamera" 0 "(bIgnoreAllPressedKeysUntilRelease=True,bForceImmediately=False,bNotifyUserSettings=False)")
      (Variables|Location|SetLocation_Desired (Transformation|GetActorLocation))
      (Variables|Zoom|SetZoom_Desired (Variables|/Script/Engine.SpringArmComponent|GetTargetArmLength (Variables|Default|GetSpringArm)))
      (Variables|Rotation|SetRotation_Desired (Transformation|GetActorRotation)))))

(event Input|MouseEvents|RightMouseButton
  (params (Key :type Key%20Structure :default "None"))
  (:Pressed
    (Utilities|FlowControl|Gate true) ; enters at Open
  )
  (:Released
    (Utilities|FlowControl|Gate true) ; enters at Close
  ))

(fn ConstructionScript)