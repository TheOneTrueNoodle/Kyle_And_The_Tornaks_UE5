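; BP_Unit is a unit actor that takes its skeletal mesh and animation class from UnitData in the construction script.
; Hover and selection setters feed a shared update that drives the ColorMultiply material parameter, tinting selected units blue and brightening hovered or selected ones.
; BeginPlay runs an endless delayed test loop that cycles through animation states and sends each to the anim instance via a message call.
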(event EventBeginPlay
  (Utilities|FlowControl|Delay 3.0 :!label _label)
  (bind _output_get (Variables|Default|SetTestAnimIndex (Utilities|Enum|ByteToEnumE_UnitAnimationState (Class|KismetMathLibrary|PercentByteByte (+ (Variables|Default|GetTestAnimIndex) 1) 6))))
  (Class|BPIUnitAnimation|SetUnitAnimationState(Message) (Components|SkeletalMesh|GetAnimInstance (Variables|Default|GetSkeletalMesh)) _output_get)
  (goto _label))

(fn ConstructionScript
  (bind _skeletalmesh (Variables|Default|GetSkeletalMesh))
  (Components|SkeletalMesh|SetSkeletalMeshAsset _skeletalmesh (Variables|/Game/Core/Units/BDA_UnitData.BDA_UnitData_C|GetSkeletalMesh (Variables|Default|GetUnitData)))
  (Class|SkeletalMeshComponent|SetAnimClass _skeletalmesh (Variables|/Game/Core/Units/BDA_UnitData.BDA_UnitData_C|GetAnimation%20Instance (Variables|Default|GetUnitData))))

(fn UpdateVisualifHoveredorSelected
  (Rendering|Material|SetVectorParameterValueonMaterials (Variables|Default|GetSkeletalMesh) "ColorMultiply" (Math|Conversions|ToVector(LinearColor) (* (* (Math|Color|SelectColor "(R=0.094118,G=0.486275,B=1.000000,A=1.000000)" "(R=1.000000,G=1.000000,B=1.000000,A=1.000000)" (Variables|Default|GetIsSelected)) (Math|Float|SelectFloat 4.0 1.0 (Variables|Default|GetIsHovered))) (Math|Float|SelectFloat 4.0 1.0 (Variables|Default|GetIsSelected))))))

(fn SetIsHovered
  (params (Hovered :type Boolean))
  (Variables|Default|SetIsHovered Hovered)
  (CallFunction|UpdateVisualifHoveredorSelected))

(fn SetIsSelected
  (params (Selected :type Boolean))
  (Variables|Default|SetIsSelected Selected)
  (CallFunction|UpdateVisualifHoveredorSelected))